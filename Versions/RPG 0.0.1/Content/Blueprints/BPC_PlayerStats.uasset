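; Player stats component that tracks health, maximum health and XP for the third-person character.
; On BeginPlay it caches its owner as BP_ThirdPersonCharacter to reach that character's HUD widget.
; Functions lower health (returning true at zero or below), heal up to the maximum, or raise the maximum, each refreshing the health bar and text.
; XP gain only adds to the stored value, with no HUD update.
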(event `self.ReceiveBeginPlay`
  (bind _asbp_third_person_character (cast `/Game/ThirdPerson/Blueprints/BP_ThirdPersonCharacter` (`self.GetOwner`)))
  (set `self.Player Character BP` _asbp_third_person_character))

(fn `Bajar Vida`
  (params (`Vida Reducida` :type "Float (double-precision)"))
  (returns (`Is Player Dead` :type Boolean))
  (bind _hud_widget (`/Game/ThirdPerson/Blueprints/BP_ThirdPersonCharacter.HUD Widget` (`self.Player Character BP`)))
  (bind _output_get (set `self.Vida Actual` (- (`self.Vida Actual`) `Vida Reducida`)))
  (`ProgressBar.SetPercent` (`/Game/UI/WB_HUD.HealthBar` _hud_widget) (/ _output_get (`self.Vida Total`)))
  (set `TextBlock.Text` (`KismetTextLibrary.Conv_DoubleToText` (`self.Vida Actual`) "HalfToEven") (`/Game/UI/WB_HUD.HealthText` _hud_widget))
  (if (<= (`self.Vida Actual`) 0.0)
    (return true)
    (else
      (return false))))

(fn `Subir Vida`
  (params (`Aumento de Vida` :type "Float (double-precision)"))
  (bind _vida_total (`self.Vida Total`))
  (bind _hud_widget (`/Game/ThirdPerson/Blueprints/BP_ThirdPersonCharacter.HUD Widget` (`self.Player Character BP`)))
  (set `self.Vida Actual` (+ (`self.Vida Actual`) `Aumento de Vida`))
  (if (> (`self.Vida Actual`) (`self.Vida Total`))
    (set `self.Vida Actual` _vida_total))
  (`ProgressBar.SetPercent` (`/Game/UI/WB_HUD.HealthBar` _hud_widget) (/ (`self.Vida Actual`) _vida_total))
  (set `TextBlock.Text` (`KismetTextLibrary.Conv_DoubleToText` (`self.Vida Actual`) "HalfToEven") (`/Game/UI/WB_HUD.HealthText` _hud_widget)))

(fn `Subir Vida Maxima`
  (params (`Aumento de Vida Maxima` :type "Float (double-precision)"))
  (bind _hud_widget (`/Game/ThirdPerson/Blueprints/BP_ThirdPersonCharacter.HUD Widget` (`self.Player Character BP`)))
  (set `self.Vida Total` (+ (`self.Vida Total`) `Aumento de Vida Maxima`))
  (`ProgressBar.SetPercent` (`/Game/UI/WB_HUD.HealthBar` _hud_widget) (/ (`self.Vida Actual`) (`self.Vida Total`)))
  (set `TextBlock.Text` (`KismetTextLibrary.Conv_DoubleToText` (`self.Vida Actual`) "HalfToEven") (`/Game/UI/WB_HUD.HealthText` _hud_widget)))

(fn `Subir XP`
  (params (`Aumento de XP` :type "Float (double-precision)"))
  (set `self.XP` (+ (`self.XP`) `Aumento de XP`)))