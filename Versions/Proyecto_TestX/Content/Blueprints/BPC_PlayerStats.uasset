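; Player stats component for BP_ThirdPersonCharacter that tracks health, experience and level, pushing changes straight to the owner's HUD widget.
; BajarVida and SubirVida clamp health, with BajarVida reporting death, while SubirVidaMaxima raises the cap.
; AñadirXP loops through level-ups, carrying surplus XP and scaling the threshold more gently past level 20.
; Each level-up also sets health to the boolean VidaActual == VidaTotal as a number, not a refill.
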(event `self.ReceiveBeginPlay`
  (bind _asbp_third_person_character (cast `/Game/ThirdPerson/Blueprints/BP_ThirdPersonCharacter` (`self.GetOwner`)))
  (set `self.Player Character BP` _asbp_third_person_character))

(fn `Añadir XP`
  (params (`Aumento de XP` :type "Float (double-precision)"))
  (bind _hud_widget (`/Game/ThirdPerson/Blueprints/BP_ThirdPersonCharacter.HUD Widget` (`self.Player Character BP`)))
  (bind _output_get (set `self.ExperienciaActual` (+ `Aumento de XP` (`self.ExperienciaActual`))))
  (while (>= (`self.ExperienciaActual`) (`self.ExperienciaMaxima`))
    (set `self.ExperienciaActual` (- (`self.ExperienciaActual`) (`self.ExperienciaMaxima`)))
    ; Subir 1 LVL
    (bind _output_get_2 (set `self.Nivel` (+ (`self.Nivel`) 1)))
    ; Texto Barra XP
    (`TextBlock.SetText` (`/Game/User_Interface/WBP/WBP_Player_Hud.TXT_Experiencia` _hud_widget) (`KismetTextLibrary.Conv_IntToText` _output_get_2))
    ; Aug, Exp, Necesaria
    (set `self.ExperienciaMaxima` (* (`self.ExperienciaMaxima`) (`KismetMathLibrary.SelectFloat` 1.125 1.2 (> (`self.Nivel`) 20))))
    ; Recompensa de Vida
    (set `self.Vida Actual` (`KismetMathLibrary.Conv_BoolToDouble` (== (`self.Vida Actual`) (`self.Vida Total`))))
    (`ProgressBar.SetPercent` (`/Game/User_Interface/WBP/WBP_Player_Hud.PB_Experiencia` _hud_widget) (/ _output_get (`self.ExperienciaMaxima`)) :!label _label))
  (goto _label))

(fn `Bajar Vida`
  (params (Cantidad :type "Float (double-precision)"))
  (returns (`Is Player Dead?` :type Boolean))
  (bind _hud_widget (`/Game/ThirdPerson/Blueprints/BP_ThirdPersonCharacter.HUD Widget` (`self.Player Character BP`)))
  (bind _output_get (set `self.Vida Actual` (`KismetMathLibrary.FClamp` (- (`self.Vida Actual`) Cantidad) 0.0 (`self.Vida Total`))))
  (`ProgressBar.SetPercent` (`/Game/User_Interface/WBP/WBP_Player_Hud.PB_Vida` _hud_widget) (/ _output_get (`self.Vida Total`)))
  (`TextBlock.SetText` (`/Game/User_Interface/WBP/WBP_Player_Hud.TXT_Vida` _hud_widget) (`KismetTextLibrary.Conv_DoubleToText` (`self.Vida Actual`) "HalfToEven"))
  (if (<= (`self.Vida Actual`) 0.0)
    (return true)
    (else
      (return false))))

(fn `Subir Vida`
  (params (`Aumento de Vida` :type "Float (double-precision)"))
  (bind _hud_widget (`/Game/ThirdPerson/Blueprints/BP_ThirdPersonCharacter.HUD Widget` (`self.Player Character BP`)))
  (set `self.Vida Actual` (`KismetMathLibrary.FClamp` (+ (`self.Vida Actual`) `Aumento de Vida`) 0.0 (`self.Vida Total`)))
  (if (> (`self.Vida Actual`) (`self.Vida Total`))
    (set `self.Vida Actual` (`self.Vida Total`)))
  (`ProgressBar.SetPercent` (`/Game/User_Interface/WBP/WBP_Player_Hud.PB_Vida` _hud_widget) (/ (`self.Vida Actual`) (`self.Vida Total`)))
  (`TextBlock.SetText` (`/Game/User_Interface/WBP/WBP_Player_Hud.TXT_Vida` _hud_widget) (`KismetTextLibrary.Conv_DoubleToText` (`self.Vida Actual`) "HalfToEven")))

(fn `Subir Vida Maxima`
  (params (Cantidad :type "Float (double-precision)"))
  (bind _hud_widget (`/Game/ThirdPerson/Blueprints/BP_ThirdPersonCharacter.HUD Widget` (`self.Player Character BP`)))
  (set `self.Vida Total` (+ (`self.Vida Total`) Cantidad))
  (`ProgressBar.SetPercent` (`/Game/User_Interface/WBP/WBP_Player_Hud.PB_Vida` _hud_widget) (/ (`self.Vida Actual`) (`self.Vida Total`)))
  (`TextBlock.SetText` (`/Game/User_Interface/WBP/WBP_Player_Hud.TXT_Vida` _hud_widget) (`KismetTextLibrary.Conv_DoubleToText` (`self.Vida Actual`) "HalfToEven")))